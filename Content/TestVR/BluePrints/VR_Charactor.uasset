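; VR test player character with axis-driven movement and look, arc teleporting, door opening and widget clicking.
; Holding 2 predicts a projectile path from Arrow1 each tick, and release teleports to its hit location.
; Right mouse line-traces for a CubeVR and activates its RotatingMovement, then on release reverses it briefly before stopping.
; Key 1 acts as a left-click through WidgetInteraction.
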(event `InputAxis|Turn`
  (params (AxisValue :type "Float (single-precision)"))
  (`self.AddControllerYawInput` AxisValue))

(event `InputAxis|TurnRate`
  (params (AxisValue :type "Float (single-precision)"))
  (`self.AddControllerPitchInput` AxisValue))

(event `InputAxis|MoveRight`
  (params (AxisValue :type "Float (single-precision)"))
  (`self.AddMovementInput` (`self.GetActorRightVector` (`GameplayStatics.GetPlayerCharacter` 0)) AxisValue))

(event `InputAxis|MoveForward`
  (params (AxisValue :type "Float (single-precision)"))
  (`self.AddMovementInput` (`self.GetActorForwardVector` (`GameplayStatics.GetPlayerCharacter` 0)) AxisValue))

(event `self.ReceiveTick`
  (params (DeltaSeconds :type "Float (single-precision)"))
  (if (`self.Is Teleport`)
    (`self.Teleport Trace`)))

(event `Key|RightMouseButton`
  (params (Key :type "Key Structure")))

(event `Key|Two`
  (params (Key :type "Key Structure"))
  (:`Pressed`
    (set `self.Is Teleport` true))
  (:`Released`
    (set `self.Is Teleport` false)
    (`self.K2_TeleportTo` (`self.LocationTrace`) (`self.K2_GetActorRotation`))))

(event `Teleport Trace`
  (bind _arrow1 (`self.Arrow1`))
  (bind _outhit (`GameplayStatics.Blueprint_PredictProjectilePath_ByTraceChannel` :`StartPos` (`SceneComponent.K2_GetComponentLocation` _arrow1) :`LaunchVelocity` (* (`SceneComponent.GetForwardVector` _arrow1) 1000.0) :`TraceChannel` "ECC_WorldStatic" :`DrawDebugType` "ForDuration"))
  (set `self.LocationTrace` (`.Location` (`GameplayStatics.BreakHitResult` _outhit))))

(event `OpenDoor`
  (bind _arrow1 (`self.Arrow1`))
  (bind _outhit (`KismetSystemLibrary.LineTraceSingleForObjects` :`Start` (`SceneComponent.K2_GetComponentLocation` _arrow1) :`End` (+ (* (`SceneComponent.GetForwardVector` _arrow1) 1000.0) (0.0 0.0 0.0)) :`ObjectTypes` (`|MakeArray` "ObjectTypeQuery1" :!type "EObjectTypeQuery Enum") :`DrawDebugType` "ForDuration"))
  (bind _ascube_vr (cast `/Game/TestVR/BluePrints/CubeVR` (`.HitActor` (`GameplayStatics.BreakHitResult` _outhit))))
  (bind _output_get (set `self.CubeVR` _ascube_vr))
  (bind _rotatingmovement (`/Game/TestVR/BluePrints/CubeVR.RotatingMovement` _output_get))
  (set `RotatingMovementComponent.RotationRate` (struct :`Yaw` -45.0) _rotatingmovement)
  (`/Engine/EditorBlueprintResources/StandardMacros.IsValid` _rotatingmovement
    (:`Is Valid`
      (`ActorComponent.SetActive` _rotatingmovement (`self.IS Active`) false))))

(event `Key|RightMouseButton`
  (params (Key :type "Key Structure"))
  (bind _cubevr (`self.CubeVR`))
  (bind _rotatingmovement (`/Game/TestVR/BluePrints/CubeVR.RotatingMovement` _cubevr))
  (:`Pressed`
    (set `self.IS Active` true)
    (`self.OpenDoor`))
  (:`Released`
    (set `self.IS Active` true)
    (`/Engine/EditorBlueprintResources/StandardMacros.IsValid` _cubevr
      (:`Is Valid`
        (set `RotatingMovementComponent.RotationRate` (struct :`Yaw` 45.0) _rotatingmovement)
        (`ActorComponent.SetActive` _rotatingmovement (`self.IS Active`) false)
        (`KismetSystemLibrary.Delay` 0.2)
        (`ActorComponent.SetActive` _rotatingmovement false false)))))

(event `Key|One`
  (params (Key :type "Key Structure"))
  (bind _widgetinteraction (`self.WidgetInteraction`))
  (:`Pressed`
    (`WidgetInteractionComponent.PressPointerKey` _widgetinteraction "LeftMouseButton"))
  (:`Released`
    (`WidgetInteractionComponent.ReleasePointerKey` _widgetinteraction "LeftMouseButton")))

(fn `UserConstructionScript`)