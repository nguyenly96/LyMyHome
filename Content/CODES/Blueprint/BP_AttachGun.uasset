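; BP_AttachGun is a gun Blueprint that displays health, armor and bullet count on its own components.
; At BeginPlay it caches the UI_Bullet widget from its widget component.
; UpdateGunUI writes the bullet count to that widget and drives inner (HP) and outer (armor) circle material parameters on a plane.
; Both circle values use a clamped, inverted remap against MaxHP and MaxArmor.
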(event `self.ReceiveBeginPlay`
  (bind _asui_bullet (cast `/Game/CODES/Blueprint/UI_Bullet` (`WidgetComponent.GetUserWidgetObject` (`self.Widget`))))
  (set `self.UI Bullet` _asui_bullet))

(event `Update GunUI`
  (params (`Current HP` :type "Float (double-precision)") (`Current Armor` :type "Float (double-precision)") (`Current Bullet` :type Integer))
  (set `/Game/CODES/Blueprint/UI_Bullet.Bullet Number` `Current Bullet` (`self.UI Bullet`))
  (`MeshComponent.SetScalarParameterValueOnMaterials` (`self.Plane`) "LoadingInnerCircle" (`KismetMathLibrary.MapRangeClamped` `Current HP` (`self.MaxHP`) 0.0 -0.01 1.0))
  (`MeshComponent.SetScalarParameterValueOnMaterials` (`self.Plane`) "LoadingIOuterCircle" (`KismetMathLibrary.MapRangeClamped` `Current Armor` (`self.MaxArmor`) 0.0 -0.01 1.0)))

(fn `UserConstructionScript`)