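; Enemy AI character that wanders the navmesh and shoots at the player.
; While idle it chains random nearby moves; a SphereView overlap makes it face the player every tick, approach, then fire BP_EnemyBullet at random intervals until overlap ends.
; Damage updates its HP widget, and at zero health it explodes and is destroyed.
; PawnSensing only prints activation changes, and FixRotate is referenced only by disconnected logic.
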(event `self.ReceiveBeginPlay`
  (bind _asui_enemy_hp (cast `/Game/CODES/Blueprint/UI_EnemyHP` (`WidgetComponent.GetUserWidgetObject` (`self.HP`))))
  (`/Engine/EditorBlueprintResources/StandardMacros.IsValid` _asui_enemy_hp
    (:`Is Valid`
      (bind _output_get (set `self.UI Enemy HP` _asui_enemy_hp))
      (set `/Game/CODES/Blueprint/UI_EnemyHP.EnemyHP` (`self.EnemyHP`) _output_get)
      (set `self.CurrentHP` (`self.EnemyHP`))
      (`KismetSystemLibrary.Delay` 1.0)
      (`self.Move to RandomPoint`))))

(event `self.ReceiveTick`
  (params (DeltaSeconds :type "Float (single-precision)"))
  (if (`self.SeePlayer`)
    (`self.Rotate and Attack Player`)))

(event `Move to RandomPoint`
  (bind _output_get (set `self.RandomLocation` (`NavigationSystemV1.K2_GetRandomLocationInNavigableRadius` (`self.K2_GetActorLocation`) 500.0 null null)))
  (`|AIMoveTo` self _output_get null
    (:`OnSuccess`
      (`KismetSystemLibrary.Delay` 1.0)
      (if (not (`self.SeePlayer`))
        (`self.Move to RandomPoint`)))))

(event `Rotate and Attack Player`
  (`self.K2_SetActorRotation` (`KismetMathLibrary.FindLookAtRotation` (`self.K2_GetActorLocation`) (`self.K2_GetActorLocation` (`self.MyCharacter`)))))

(event `self.SphereView.OnComponentBeginOverlap`
  (params (OverlappedComponent :type "PrimitiveComponent Object Reference") (OtherActor :type "Actor Object Reference") (OtherComp :type "PrimitiveComponent Object Reference") (OtherBodyIndex :type Integer) (bFromSweep :type Boolean) (SweepResult :type "HitResult Structure (by ref)"))
  (`/Engine/EditorBlueprintResources/StandardMacros.IsValid` (`self.MyCharacter`)
    (:`Is Not Valid`
      (bind _asmy_character (cast `/Game/CODES/Blueprint/MyCharacter` OtherActor))
      (`/Engine/EditorBlueprintResources/StandardMacros.IsValid` _asmy_character
        (:`Is Valid`
          (set `self.MyCharacter` _asmy_character)
          (set `self.SeePlayer` true)
          (`|AIMoveTo` self (0.0 0.0 0.0) (`self.MyCharacter`) 100.0 true
            (:`OnSuccess`
              (`self.Enemy Attack`))))))))

(event `self.SphereView.OnComponentEndOverlap`
  (params (OverlappedComponent :type "PrimitiveComponent Object Reference") (OtherActor :type "Actor Object Reference") (OtherComp :type "PrimitiveComponent Object Reference") (OtherBodyIndex :type Integer))
  (bind _mycharacter (`self.MyCharacter`))
  (`/Engine/EditorBlueprintResources/StandardMacros.IsValid` _mycharacter
    (:`Is Valid`
      (if (== OtherActor _mycharacter)
        (cast `/Game/CODES/Blueprint/MyCharacter` OtherActor)
        (set `self.MyCharacter` null)
        (set `self.SeePlayer` false)
        (`self.Move to RandomPoint`)))))

(event `Enemy Attack`
  (if (`self.SeePlayer`)
    (`|SpawnActorFromClass` "/Game/CODES/Blueprint/BP_EnemyBullet.BP_EnemyBullet_C" (`SceneComponent.K2_GetComponentToWorld` (`self.BulletSpawnLocation`)) "Undefined" "OverrideRootScale" null (`self.Bullet Speed`) (`self.Bullet Dame`) null)
    (`KismetSystemLibrary.Delay` (`KismetMathLibrary.RandomFloatInRange` 0.2 (`self.Delay Between 2 Amor`)))
    (`self.Enemy Attack`)))

(event `TakeDamage`
  (params (B :type "Float (double-precision)"))
  (bind _returnvalue (`SceneComponent.K2_GetComponentLocation` (`self.Body`)))
  (bind _output_get (set `self.CurrentHP` (- (`self.CurrentHP`) B)))
  (`/Game/CODES/Blueprint/UI_EnemyHP.Update HP` (`self.UI Enemy HP`) _output_get)
  (if (<= (`self.CurrentHP`) 0.0)
    (`SceneComponent.SetVisibility` (`self.Body`) false false)
    (`GameplayStatics.SpawnEmitterAtLocation` "/Game/InfinityBladeEffects/Effects/FX_Monsters/FX_Monster_Gruntling/Notifies/P_Death_backpack_expl.P_Death_backpack_expl" _returnvalue (struct) (1.5 1.5 1.5))
    (`GameplayStatics.SpawnSoundAtLocation` "/Game/ProSoundCollection/ExplosionFireGas/Wavs/explosion_large_no_tail_05.explosion_large_no_tail_05" _returnvalue (struct) 1.0 1.0 0.0 null null)
    (`self.K2_DestroyActor`)))

(event `self.PawnSensing.OnSeePawn`
  (params (Pawn :type "Pawn Object Reference")))

(event `self.PawnSensing.OnComponentActivated`
  (params (Component :type "ActorComponent Object Reference") (bReset :type Boolean))
  (`KismetSystemLibrary.PrintString` "Activated"))

(event `self.PawnSensing.OnComponentDeactivated`
  (params (Component :type "ActorComponent Object Reference"))
  (`KismetSystemLibrary.PrintString` "Deactivated"))

(fn `FixRotate`
  (params (Target :type "Vector Structure (by ref)"))
  (returns (ReturnValue :type "Rotator Structure"))
  (bind (_returnvalue_roll _returnvalue_pitch) (`KismetMathLibrary.BreakRotator` (`self.K2_GetActorRotation`)))
  (`SceneComponent.K2_SetWorldRotation` (`self.Body`) (`KismetMathLibrary.FindLookAtRotation` (`SceneComponent.K2_GetComponentLocation` (`self.Body`)) (`SceneComponent.K2_GetComponentLocation` (`/Game/CODES/Blueprint/MyCharacter.FirstPersonCamera` (`self.MyCharacter`)))) false false)
  (return (`KismetMathLibrary.MakeRotator` _returnvalue_roll _returnvalue_pitch (.yaw (`KismetMathLibrary.FindLookAtRotation` (`self.K2_GetActorLocation`) Target)))))

(fn `UserConstructionScript`
  (set `CharacterMovementComponent.MaxWalkSpeed` (`self.Move Speed`) (`self.CharacterMovement`)))